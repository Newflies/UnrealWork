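; BP_SWeapon is a weapon Blueprint that adds laser-shot effects to firing and removes itself when it has no owner.
; HandFire calls the parent implementation, attaches a bullet-trail Niagara system to its Niagara component, and plays a laser sound at half volume at the mesh's location.
; Tick checks the owner every frame and destroys the actor once that owner is invalid.
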(event EventBeginPlay)

(event Collision|EventActorBeginOverlap
  (params (OtherActor :type Actor%20Object%20Reference)))

(event EventTick
  (params (DeltaSeconds :type Float%20%28single-precision%29))
  (Utilities|IsValid (Components|GetOwner self)
    (:Is%20Not%20Valid
      (Actor|DestroyActor))))

(event EventHandFire
  (bind _meshcomp (Variables|Default|GetMeshComp))
  (bind _returnvalue (Transformation|GetWorldTransform _meshcomp))
  (|CallParentFunction)
  (Niagara|SpawnSystemAttached "/Game/sA_ShootingVfxPack/FX/NiagaraSystems/NS_BulletTrail_1.NS_BulletTrail_1" (Variables|Default|GetNiagara) "None" "0, 0, 0" "0, 0, 0" "KeepRelativeOffset" false)
  (Audio|PlaySoundatLocation "/Game/Sound/激光射击.激光射击" (.location _returnvalue) (.rotation _returnvalue) 0.5 1.0 0.0 0 0 0))

(fn ConstructionScript)