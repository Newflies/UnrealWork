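; Player controller Blueprint that owns the local player's HUD and in-game menu widgets.
; ClientPostLogin calls SetupIngameUI, which creates both widgets for local controllers but adds only the HUD to the viewport.
; ShowInGameMenu and HideInGameMenu attach or remove the menu, switching input between UI-only and game-only.
; The GameMode cast after setup leads nowhere, and the event graph's ShowInGameMenu and RespawnPlayerEvent calls are unwired.
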(event Custom|ClientPostLogin
  (CallFunction|SetupIngameUI)
  (Utilities|Casting|CastToMyFDEMOGameMode (Game|GetGameMode)))

(event EventEndPlay
  (params (EndPlayReason :type EEndPlayReason%20Enum :default "Destroyed")))

(fn ConstructionScript)

(fn SetupIngameUI
  (if (Pawn|IsLocalPlayerController)
    (bind _returnvalue (UserInterface|CreateWidget "/Game/BluePrints/Widgets/MyHUD.MyHUD_C" self))
    (Variables|Default|SetHUDWidget _returnvalue)
    (UserInterface|Viewport|AddtoViewport (Variables|Default|GetHUDWidget) 0)
    (bind _returnvalue_2 (UserInterface|CreateWidget "/Game/BluePrints/Widgets/InGameMenu.InGameMenu_C" self))
    (Variables|Default|SetInGameMenuWidget _returnvalue_2)))

(fn ShowinGameMenu
  (bind _ingamemenuwidget (Variables|Default|GetInGameMenuWidget))
  (UserInterface|Viewport|AddtoViewport _ingamemenuwidget 0)
  (Input|SetInputModeUIOnly self _ingamemenuwidget "DoNotLock"))

(fn HideinGameMenu
  (Widget|RemovefromParent (Variables|Default|GetInGameMenuWidget))
  (Input|SetInputModeGameOnly self))