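; MyTarget is a target actor that awards score when it is hit.
; The Hit event calls AddScore, which casts the first entry in the GameState's PlayerArray to MyPlayerState, increments its score and prints a success message, regardless of who caused the hit.
; BeginPlay also requests a looping zero-interval timer for UpdateTimer, whose only content is an empty, always-false branch.
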(event Custom|UpdateTimer
  (if (> 0 0)
    _))

(event EventBeginPlay
  (Utilities|Time|SetTimerbyEvent (delegate Custom|UpdateTimer) 0.0 true))

(event Collision|EventActorBeginOverlap
  (params (OtherActor :type Actor%20Object%20Reference)))

(event Collision|EventHit
  (params (MyComp :type Primitive%20Component%20Object%20Reference) (Other :type Actor%20Object%20Reference) (OtherComp :type Primitive%20Component%20Object%20Reference) (bSelfMoved :type Boolean) (HitLocation :type Vector :default "0, 0, 0") (HitNormal :type Vector :default "0, 0, 0") (NormalImpulse :type Vector :default "0, 0, 0") (Hit :type Hit%20Result%20Structure%20%28by%20ref%29))
  (CallFunction|AddScore))

(fn ConstructionScript)

(fn AddScore
  (bind _returnvalue (Game|GetGameState))
  (Utilities|IsValid _returnvalue
    (:Is%20Valid
      (for _array_element (Variables|/Script/Engine.GameStateBase|GetPlayerArray _returnvalue)
        (bind _asmy_player_state (Utilities|Casting|CastToMyPlayerState _array_element))
        (Default|IncrementScore _asmy_player_state)
        (Development|PrintString "添加分数成功")
        (return)))))