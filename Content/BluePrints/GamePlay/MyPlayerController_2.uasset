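; Player controller Blueprint that owns the local player's HUD, in-game menu and rank list widgets.
; On ClientPostLogin it creates all three for the local controller and adds only the HUD to the viewport.
; The OpenInGameMenu input shows the menu with UI-only input and a visible cursor.
; Paired show and hide functions toggle the menu and rank list, restoring game-only input on hide.
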(event Custom|ClientPostLogin
  (CallFunction|SetupIngameUI)
  (Utilities|Casting|CastToMyFDEMOGameMode (Game|GetGameMode)))

(event EventEndPlay
  (params (EndPlayReason :type EEndPlayReason%20Enum :default "Destroyed")))

(event Input|ActionEvents|InputActionOpenInGameMenu
  (params (Key :type Key%20Structure :default "None"))
  (:Pressed
    (CallFunction|ShowinGameMenu)
    (Variables|Default|SetbShowMouseCursor true)))

(fn ConstructionScript)

(fn SetupIngameUI
  (if (Pawn|IsLocalPlayerController)
    (bind _returnvalue (UserInterface|CreateWidget "/Game/BluePrints/Widgets/MyHUD.MyHUD_C" self))
    (Variables|Default|SetHUDWidget _returnvalue)
    (UserInterface|Viewport|AddtoViewport (Variables|Default|GetHUDWidget) 0)
    (bind _returnvalue_2 (UserInterface|CreateWidget "/Game/BluePrints/Widgets/InGameMenu.InGameMenu_C" self))
    (Variables|Default|SetInGameMenuWidget _returnvalue_2)
    (bind _returnvalue_3 (UserInterface|CreateWidget "/Game/BluePrints/Widgets/RankList.RankList_C" self))
    (Variables|Default|SetRankListWidget _returnvalue_3)))

(fn ShowinGameMenu
  (bind _ingamemenuwidget (Variables|Default|GetInGameMenuWidget))
  (UserInterface|Viewport|AddtoViewport _ingamemenuwidget 0)
  (Input|SetInputModeUIOnly self _ingamemenuwidget "LockAlways")
  (Variables|Default|SetbShowMouseCursor true))

(fn HideinGameMenu
  (Widget|RemovefromParent (Variables|Default|GetInGameMenuWidget))
  (Input|SetInputModeGameOnly self)
  (Variables|Default|SetbShowMouseCursor false))

(fn SetupRankList
  (bind _ranklistwidget (Variables|Default|GetRankListWidget))
  (UserInterface|Viewport|AddtoViewport _ranklistwidget 0)
  (Input|SetInputModeUIOnly self _ranklistwidget "DoNotLock"))

(fn HideinRankList
  (Widget|RemovefromParent (Variables|Default|GetRankListWidget))
  (Input|SetInputModeGameOnly self))