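; Game mode for a two-player multiplayer demo that registers joining players and respawns their characters at per-player starts.
; On login, the server sorts PlayerStarts into Player1 and Player2 lists by tag, numbers the player for consistent scoreboard order and calls the controller's ClientPostLogin.
; RespawnPlayerEvent destroys the current pawn, then spawns and possesses a ThirdPersonCharacter at the first Player1 start for the first PlayerArray entry, otherwise the first Player2 start.
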(event Custom|RespawnPlayerEvent
  (params (Player%20Controller :type Player%20Controller%20Object%20Reference))
  (bind _returnvalue (Pawn|GetControlledPawn Player%20Controller))
  (Utilities|IsValid _returnvalue
    (:Is%20Valid
      (Actor|DestroyActor _returnvalue))
    (:Is%20Not%20Valid
      _))
  (if (== (Variables|/Script/Engine.PlayerState|GetPlayerId (Variables|/Script/Engine.Controller|GetPlayerState Player%20Controller)) (Variables|/Script/Engine.PlayerState|GetPlayerId (Utilities|Array|Get(acopy) (Variables|/Script/Engine.GameStateBase|GetPlayerArray (Game|GetGameState)))))
    (bind _returnvalue_2 (Game|SpawnActorfromClass "/Game/ThirdPersonCPP/Blueprints/ThirdPersonCharacter.ThirdPersonCharacter_C" (Transformation|GetActorTransform (Utilities|Array|Get(acopy) (Variables|Default|GetPlayer1))) "AdjustIfPossibleButDontSpawnIfColliding" 0 0))
    (Pawn|Possess Player%20Controller _returnvalue_2)
    (else
      (bind _returnvalue_3 (Game|SpawnActorfromClass "/Game/ThirdPersonCPP/Blueprints/ThirdPersonCharacter.ThirdPersonCharacter_C" (Transformation|GetActorTransform (Utilities|Array|Get(acopy) (Variables|Default|GetPlayer2))) "AdjustIfPossibleButDontSpawnIfColliding" 0 0))
      (Pawn|Possess Player%20Controller _returnvalue_3))))

(event EventBeginPlay)

(event EventTick
  (params (DeltaSeconds :type Float%20%28single-precision%29)))

(event EventPostLogin
  (params (NewPlayer :type Player%20Controller%20Object%20Reference))
  (Networking|SwitchHasAuthority
    (:Authority
      (bind _outactors (Actor|GetAllActorsOfClass "/Script/Engine.PlayerStart"))
      (for _array_element _outactors
        (if (Utilities|Name|Equal(Name) (Variables|/Script/Engine.PlayerStart|GetPlayerStartTag _array_element) "Player1")
          (Utilities|Array|AddUnique (Variables|Default|GetPlayer1) _array_element)
          (else
            (Utilities|Array|AddUnique (Variables|Default|GetPlayer2) _array_element))))
      (bind _asmy_player_state (Utilities|Casting|CastToMyPlayerState (Variables|/Script/Engine.Controller|GetPlayerState NewPlayer)))
      (Variables|/Game/BluePrints/GamePlay/MyPlayerState.MyPlayerState_C|SetPlayerNumber _asmy_player_state (Utilities|Array|Length (Variables|/Script/Engine.GameState|GetPlayerArray (Game|GetGameState)))) ; Makes the scoreboard in the same order for all players
      (bind _asmy_player_controller_2 (Utilities|Casting|CastToMyPlayerController_2 NewPlayer))
      (Default|ClientPostLogin _asmy_player_controller_2))))

(fn ConstructionScript)