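; MatchTimer is a trigger Blueprint meant as a match countdown, showing its Time value as integer text on a TextRender component.
; BeginPlay and ThirdPersonCharacter hits on the text share one path, which sets TextRender to None before calling SetText on it.
; StartTimer, uncalled here, decrements Time only when Time minus one is zero or below, otherwise calling the empty EndMatch.
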(event OnComponentHit(TextRender)
  (params (HitComponent :type Primitive%20Component%20Object%20Reference) (OtherActor :type Actor%20Object%20Reference) (OtherComp :type Primitive%20Component%20Object%20Reference) (NormalImpulse :type Vector :default "0, 0, 0") (Hit :type Hit%20Result%20Structure%20%28by%20ref%29))
  (Utilities|Casting|CastToThirdPersonCharacter OtherActor)
  (bind _output_get (Variables|Default|SetTextRender 0))
  (Rendering|Components|TextRender|SetText _output_get (Utilities|Text|ToText(Integer) (Variables|Default|GetTime))))

(event EventBeginPlay
  (bind _output_get (Variables|Default|SetTextRender 0))
  (Rendering|Components|TextRender|SetText _output_get (Utilities|Text|ToText(Integer) (Variables|Default|GetTime))))

(event EventTick
  (params (DeltaSeconds :type Float%20%28single-precision%29)))

(fn ConstructionScript)

(fn EndMatch)

(fn StartTimer
  (if (<= (- (Variables|Default|GetTime) 1) 0)
    (Variables|Default|SetTime (- (Variables|Default|GetTime) 1))
    (else
      (CallFunction|EndMatch))))